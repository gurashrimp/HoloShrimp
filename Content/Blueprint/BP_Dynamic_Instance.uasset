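; BP_Dynamic_Instance is an actor that changes its mesh's color and shape when something overlaps its box.
; BeginPlay creates a dynamic material instance on the static mesh and enables player input, though no input events appear.
; Overlap begin plays a timeline driving the "Base color" parameter and swaps the mesh to a cylinder; overlap end reverses it and restores a cube.
; A flag ignores new color triggers until the timeline finishes.
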(event OnComponentEndOverlap(Box)
  (params (OverlappedComponent :type Primitive%20Component%20Object%20Reference) (OtherActor :type Actor%20Object%20Reference) (OtherComp :type Primitive%20Component%20Object%20Reference) (OtherBodyIndex :type Integer))
  ;[1 1 1] Changing Color And Mesh
  (Utilities|FlowControl|Sequence
    (:then_0
      (if (not (Variables|Default|GetChangingColor?))
        (Variables|Default|SetChangingColor? true)
        (bind _color_change (Timeline|Timeline Reverse)
          (:Update
            (Rendering|Material|SetVectorParameterValue (Variables|Default|GetNewVar) "Base color" _color_change :!class /Script/Engine.MaterialInstanceDynamic))
          (:Finished
            (Variables|Default|SetChangingColor? false)))))
    (:then_1
      (if (not (Variables|Default|GetIsShapeShifting?))
        (Variables|Default|SetIsShapeShifting? true)
        (Components|StaticMesh|SetStaticMesh (Variables|Default|GetStaticMesh) "/Engine/BasicShapes/Cube.Cube")
        (Variables|Default|SetIsShapeShifting? false)))))

(event OnComponentBeginOverlap(Box)
  (params (OverlappedComponent :type Primitive%20Component%20Object%20Reference) (OtherActor :type Actor%20Object%20Reference) (OtherComp :type Primitive%20Component%20Object%20Reference) (OtherBodyIndex :type Integer) (bFromSweep :type Boolean) (SweepResult :type Hit%20Result%20Structure%20%28by%20ref%29))
  ;[1 1 1] Changing Color And Mesh
  (Utilities|FlowControl|Sequence
    (:then_0
      (if (not (Variables|Default|GetChangingColor?))
        (Variables|Default|SetChangingColor? true)
        (bind _color_change (Timeline|Timeline PlayFromStart)
          (:Update
            (Rendering|Material|SetVectorParameterValue (Variables|Default|GetNewVar) "Base color" _color_change :!class /Script/Engine.MaterialInstanceDynamic))
          (:Finished
            (Variables|Default|SetChangingColor? false)))))
    (:then_1
      (if (Variables|Default|GetIsShapeShifting?)
        _
        (else
          (Variables|Default|SetIsShapeShifting? true)))
      (Components|StaticMesh|SetStaticMesh (Variables|Default|GetStaticMesh) "/Engine/BasicShapes/Cylinder.Cylinder")
      (Variables|Default|SetIsShapeShifting? false))))

(event EventBeginPlay
  (bind _staticmesh (Variables|Default|GetStaticMesh))
  (bind _returnvalue (Rendering|Material|CreateDynamicMaterialInstance _staticmesh 0 (Rendering|Material|GetMaterial _staticmesh 0) "None" :!class /Script/Engine.PrimitiveComponent))
  (Variables|Default|SetNewVar _returnvalue)
  (Input|EnableInput (Game|GetPlayerController 0)))

(fn ConstructionScript)